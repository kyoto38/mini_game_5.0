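; Spline-shaped power line actor that draws the line as meshes and passes power updates on to its target actor.
; The construction script clears and rebuilds one spline mesh per segment, with cross-section from scaled-down point scales and the main power material applied.
; When a power update finishes, it calls the update on TargetActor, preserving the Forced flag.
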(event `self.ReceiveBeginPlay`
  (`parent.ReceiveBeginPlay`))

(event `self.Setup Material Owners`)

(event `self.On Update Power Finished`
  (params (Forced :type Boolean))
  (`self.Update Power On Target` Forced (`self.TargetActor`)))

(event `Create Spline Area`
  (bind _spline (`self.Spline`))
  (for _array_element (`self.K2_GetComponentsByClass` "/Script/Engine.SplineMeshComponent")
    (`ActorComponent.K2_DestroyComponent` _array_element))
  (for _index (range (+ (- (`SplineComponent.GetNumberOfSplinePoints` _spline) 2) 1))
    (bind _returnvalue (`AddComponent|NODE_AddSplineMeshComponent-2`))
    (`SceneComponent.K2_AttachToComponent` _returnvalue (`self.DefaultSceneRoot`) "None" "KeepRelative" "KeepRelative" "KeepRelative" true)
    (bind (_location _tangent) (`SplineComponent.GetLocationAndTangentAtSplinePoint` _spline _index "Local"))
    (bind _returnvalue_2 (+ _index 1))
    (bind (_location_2 _tangent_2) (`SplineComponent.GetLocationAndTangentAtSplinePoint` _spline _returnvalue_2 "Local"))
    (`SplineMeshComponent.SetStartAndEnd` _returnvalue _location _tangent _location_2 _tangent_2 true)
    (`SplineMeshComponent.SetStartScale` _returnvalue (* (`KismetMathLibrary.MakeVector2D` (.y (`SplineComponent.GetScaleAtSplinePoint` _spline _index)) (.z (`SplineComponent.GetScaleAtSplinePoint` _spline _index))) 0.05) true)
    (`SplineMeshComponent.SetEndScale` _returnvalue (* (`KismetMathLibrary.MakeVector2D` (.y (`SplineComponent.GetScaleAtSplinePoint` _spline _returnvalue_2)) (.z (`SplineComponent.GetScaleAtSplinePoint` _spline _returnvalue_2))) 0.05) true)
    (`PrimitiveComponent.SetMaterial` _returnvalue 0 (`self.Main Power Material`))))

(fn `UserConstructionScript`
  (`parent.UserConstructionScript`)
  (`self.Create Spline Area`))