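; Logic gate actor that acts as a power inverter (NOT gate), reporting the opposite of its parent class's active status.
; Construction and BeginPlay create a separate material for the InPower mesh, while Sphere and OutPower share the main power material.
; During power updates the input material shows the inverse of the transition amount.
; When an update finishes, it sets that material from Active and propagates power to TargetActor.
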(event `self.ReceiveBeginPlay`
  (`self.Setup Additional Power`)
  (`parent.ReceiveBeginPlay`))

(event `self.Setup Material Owners`
  (`PrimitiveComponent.SetMaterial` (`self.Sphere`) 0 (`self.Main Power Material`))
  (`PrimitiveComponent.SetMaterial` (`self.OutPower`) 0 (`self.Main Power Material`))
  (`PrimitiveComponent.SetMaterial` (`self.InPower`) 0 (`self.InPowerMaterial`)))

(event `self.On Update Power Finished`
  (params (Forced :type Boolean))
  (`/Game/FPPTemplate/Blueprints/Core/BPFL_FPPT_Power.Update Power Material` (`self.InPowerMaterial`) (`KismetMathLibrary.Conv_BoolToDouble` (`self.Active`)) (`self.Power Type`))
  (`self.Update Power On Target` Forced (`self.Target Actor`)))

(event `self.On Update Power Update`
  (params (`Current Amount` :type "Float (single-precision)"))
  (`/Game/FPPTemplate/Blueprints/Core/BPFL_FPPT_Power.Update Power Material` (`self.InPowerMaterial`) (- 1.0 `Current Amount`) (`self.Power Type`)))

(fn `Get Active Status`
  (returns (`Current Active` :type Boolean))
  (return (not (`parent.Get Active Status`))))

(fn `Setup Additional Power`
  (bind _power_material_new (`self.Make New Power Material` (`self.Active`)))
  (set `self.InPowerMaterial` _power_material_new))

(fn `UserConstructionScript`
  (`self.Setup Additional Power`)
  (`parent.UserConstructionScript`))