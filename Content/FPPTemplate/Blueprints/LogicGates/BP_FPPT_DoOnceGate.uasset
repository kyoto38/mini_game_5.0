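; DoOnce logic gate in the FPP Template power system that latches its output after the first incoming power-on.
; With Use2PowerReset, power-off re-arms the DoOnce and each power-on flips Inverse, turning the latch into a toggle.
; Parent power update events drive the output material's animated transition and forward the resulting state, rather than the raw input, to TargetActor.
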(event `self.ReceiveBeginPlay`
  (bind _didactivate (`self.DidActivate`))
  (`self.Setup Additional Power`)
  (set `self.Activation Finished` _didactivate)
  (set `self.Inverse` (select `bool` (`self.Use2PowerReset?`) :`true` (not _didactivate)))
  (`parent.ReceiveBeginPlay`))

(event `self.Setup Material Owners`
  (`PrimitiveComponent.SetMaterial` (`self.CubeGlow`) 0 (`self.OutputMaterial`))
  (`PrimitiveComponent.SetMaterial` (`self.OutPower`) 0 (`self.OutputMaterial`))
  (`PrimitiveComponent.SetMaterial` (`self.InPower`) 0 (`self.Main Power Material`)))

(event `self.On Update Power Finished`
  (params (Forced :type Boolean))
  (`/Game/FPPTemplate/Blueprints/Core/BPFL_FPPT_Power.Update Power Material` (`self.OutputMaterial`) (`KismetMathLibrary.Conv_BoolToDouble` (`self.Get Inversed Active`)) (`self.Power Type`))
  (`self.Update Power On Target` Forced (`self.Target Actor`) true (`self.Get Inversed Active`))
  (set `self.Activation Finished` (`self.DidActivate`)))

(event `self.On Update Power Update`
  (params (`Current Amount` :type "Float (single-precision)"))
  (`/Game/FPPTemplate/Blueprints/Core/BPFL_FPPT_Power.Update Power Material` (`self.OutputMaterial`) (`KismetMathLibrary.SelectFloat` (`KismetMathLibrary.SelectFloat` 0.0 1.0 (`self.Inverse`)) (`KismetMathLibrary.SelectFloat` (- 1.0 `Current Amount`) `Current Amount` (`self.Inverse`)) (`self.Activation Finished`)) (`self.Power Type`)))

(event `/Game/FPPTemplate/Blueprints/Core/BPI_FPPT_Switchable.On Power Update`
  (params (`New Active` :type Boolean) (`Is Forced` :type Boolean) (`Intial Actor` :type "Actor Object Reference"))
  (if `New Active`
    (if (`self.Use2PowerReset?`)
      (set `self.Inverse` (not (`self.Inverse`)))
      (set `self.Activation Finished` false)
      (set `self.DidActivate` false))
    (if (not (`self.DidActivate`))
      (`/Engine/EditorBlueprintResources/StandardMacros.DoOnce` (`self.DidActivate`) :!label _label
        (:`Completed`
          (set `self.DidActivate` true))))
    (elif (`self.Use2PowerReset?`)
      (`|ExecutionSequence`
        (:`then_0`
          (goto _label :!via `Reset`))
        (:`then_1`
          _))))
  (`parent.On Power Update` `New Active` `Is Forced` `Intial Actor`))

(fn `Get Active Status`
  (returns (`Current Active` :type Boolean))
  (return (`self.Active`)))

(fn `Get Inversed Active`
  (returns (Active :type Boolean))
  (if (`self.Inverse`)
    (return (not (`self.DidActivate`)))
    (else
      (return (`self.DidActivate`)))))

(fn `Setup Additional Power`
  (bind _power_material_new (`self.Make New Power Material` (`self.Get Inversed Active`)))
  (set `self.OutputMaterial` _power_material_new))

(fn `UserConstructionScript`
  (`self.Setup Additional Power`)
  (`parent.UserConstructionScript`))