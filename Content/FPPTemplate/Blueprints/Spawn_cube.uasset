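; Trigger actor that spawns a BP_FPPT_PowerCube when the player pawn overlaps its Box.
; The overlap handler destroys the previously spawned cube and spawns a replacement at the actor's location, so it keeps one at a time.
; A Cube flag and short Delay form a cooldown between spawns.
; A separate Spawncube function, not called here, spawns at the Box's relative location.
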(event `self.Box.OnComponentBeginOverlap`
  (params (OverlappedComponent :type "PrimitiveComponent Object Reference") (OtherActor :type "Actor Object Reference") (OtherComp :type "PrimitiveComponent Object Reference") (OtherBodyIndex :type Integer) (bFromSweep :type Boolean) (SweepResult :type "HitResult Structure (by ref)"))
  (bind _returnvalue_location (`KismetMathLibrary.BreakTransform` (`self.GetTransform`)))
  (cast `/Game/FPPTemplate/Blueprints/Game/BP_FPPT_PlayerPawn` OtherActor)
  (if (not (`self.cube?`))
    (`self.K2_DestroyActor` (stale _returnvalue))
    (bind _returnvalue (`|SpawnActorFromClass` "/Game/FPPTemplate/Blueprints/BP_FPPT_PowerCube.BP_FPPT_PowerCube_C" (`KismetMathLibrary.MakeTransform` _returnvalue_location) "Undefined" "OverrideRootScale" null null))
    (set `self.cube?` true)
    (`KismetSystemLibrary.Delay` 5.0)
    (set `self.cube?` false)))

(fn `spawncube`
  (`|SpawnActorFromClass` "/Game/FPPTemplate/Blueprints/BP_FPPT_PowerCube.BP_FPPT_PowerCube_C" (`KismetMathLibrary.Conv_VectorToTransform` (`SceneComponent.RelativeLocation` (`self.Box`))) "Undefined" "OverrideRootScale" null null))

(fn `UserConstructionScript`)