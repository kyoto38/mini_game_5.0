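; A power-driven door interactable for the FPP template that grows or collapses vertically with its power state.
; Power update events feed UpdatePositions, which scales DoorAnchor on Z from zero at no power to full size at full power.
; When the update finishes, it snaps to the Active state.
; The door mesh takes MainPowerMaterial in SetupMaterialOwners.
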(event `self.ReceiveBeginPlay`
  (`parent.ReceiveBeginPlay`))

(event `self.Setup Material Owners`
  (`PrimitiveComponent.SetMaterial` (`self.Door`) 0 (`self.Main Power Material`)))

(event `self.On Update Power Update`
  (params (`Current Amount` :type "Float (single-precision)"))
  (`self.Update Positions` `Current Amount`))

(event `self.On Update Power Finished`
  (params (Forced :type Boolean))
  (`self.Update Positions` (`KismetMathLibrary.Conv_BoolToDouble` (`self.Active`))))

(fn `Update Positions`
  (params (Amount :type "Float (double-precision)"))
  (`SceneComponent.SetRelativeScale3D` (`self.DoorAnchor`) (`KismetMathLibrary.MakeVector` 1.0 1.0 (`KismetMathLibrary.Lerp` 0.0 1.0 Amount))))

(fn `UserConstructionScript`
  (`parent.UserConstructionScript`))